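; BP_B01 is a test AI-controlled Blueprint for Gianguscio, a companion-like actor whose inside-shell state can be toggled.
; On BeginPlay it registers itself in the Gianguscio variable of the player's BP_ThirdPersonCharacter.
; Its Interact event flips the InsideShell bool on its AI controller's blackboard and prints the new value for debugging.
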(event `self.ReceiveBeginPlay`
  (bind _asbp_third_person_character (cast `/Game/ThirdPerson/Blueprints/BP_ThirdPersonCharacter` (`GameplayStatics.GetPlayerCharacter` 0)))
  (set `/Game/ThirdPerson/Blueprints/BP_ThirdPersonCharacter.Gianguscio` self _asbp_third_person_character))

(event `/Game/BP_Interface.Interact`
  (bind _returnvalue (`AIBlueprintHelperLibrary.GetBlackboard` (`AIBlueprintHelperLibrary.GetAIController` self)))
  (if (`BlackboardComponent.GetValueAsBool` (`AIBlueprintHelperLibrary.GetBlackboard` (`AIBlueprintHelperLibrary.GetAIController` self)) "InsideShell")
    (`BlackboardComponent.SetValueAsBool` _returnvalue "InsideShell" false)
    (`KismetSystemLibrary.PrintString` "False")
    (else
      (`BlackboardComponent.SetValueAsBool` _returnvalue "InsideShell" true)
      (`KismetSystemLibrary.PrintString` "True"))))

(fn `UserConstructionScript`)